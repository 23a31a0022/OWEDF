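; BP_MyHero is a player character Blueprint that sets up Enhanced Input movement and camera look.
; BeginPlay adds the IMC_MyDefault mapping context to player 0's input subsystem.
; IA_MyMove adds movement along forward and right vectors built only from control-rotation yaw, so pitch does not affect direction.
; IA_MyLook feeds controller yaw and pitch, though both actions show constant zero vectors in place of action values.
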(event Input|EnhancedActionEvents|EnhancedInputActionIA_MyMove
  (params (ActionValue :type Boolean) (ElapsedSeconds :type Float%20%28double-precision%29) (TriggeredSeconds :type Float%20%28double-precision%29) (InputAction :type Input%20Action%20Object%20Reference :default "/Game/Mygame/MyIA/IA_MyMove.IA_MyMove"))
  (bind _returnvalue (Pawn|GetControlRotation :!class /Script/Engine.Pawn))
  (bind (_x _y) (Math|Vector2D|BreakVector2D))
  (bind _yaw (Math|Rotator|BreakRotator _returnvalue))
  (bind _returnvalue_2 (Math|Rotator|MakeRotator 0.0 0.0 _yaw))
  (Utilities|FlowControl|Sequence
    (:then_0
      (Pawn|Input|AddMovementInput (Math|Vector|GetForwardVector _returnvalue_2) _y false))
    (:then_1
      (Pawn|Input|AddMovementInput (Math|Vector|GetRightVector _returnvalue_2) _x false))))

(event Input|EnhancedActionEvents|EnhancedInputActionIA_MyLook
  (params (ActionValue :type Boolean) (ElapsedSeconds :type Float%20%28double-precision%29) (TriggeredSeconds :type Float%20%28double-precision%29) (InputAction :type Input%20Action%20Object%20Reference :default "/Game/Mygame/MyIA/IA_MyLook.IA_MyLook"))
  (bind (_x _y) (Math|Vector2D|BreakVector2D))
  (Utilities|FlowControl|Sequence
    (:then_0
      (Pawn|Input|AddControllerYawInput _x))
    (:then_1
      (Pawn|Input|AddControllerPitchInput _y))))

(event EventBeginPlay
  (Input|AddMappingContext (PlayerController|LocalPlayerSubsystems|GetEnhancedInputLocalPlayerSubsystem (Game|GetPlayerController 0)) "/Game/Mygame/MyIA/IMC_MyDefault.IMC_MyDefault" 0 "(bIgnoreAllPressedKeysUntilRelease=True,bForceImmediately=False,bNotifyUserSettings=False)"))

(fn ConstructionScript)