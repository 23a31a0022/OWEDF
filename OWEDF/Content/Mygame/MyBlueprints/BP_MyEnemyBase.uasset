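; BP_MyEnemyBase is an enemy base that chases the player and can be killed by damage.
; From BeginPlay, an AIMoveTo call heads for player character 0 and repeats after a short delay on success or failure, forming an endless pursuit loop.
; AnyDamage subtracts from Health and destroys the actor once it reaches zero or below.
; Debug prints show each loop pass and the remaining Health.
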(event EventBeginPlay
  (Development|PrintString "Hello" :!label _label)
  (AI|AIMoveTo self "0, 0, 0" (Game|GetPlayerCharacter 0) 5e+01 false
    (:OnSuccess
      (Utilities|FlowControl|Delay 0.5)
      (goto _label))
    (:OnFail
      (Utilities|FlowControl|Delay 0.5)
      (goto _label))))

(event Game|Damage|EventAnyDamage
  (params (Damage :type Float%20%28single-precision%29) (DamageType :type Damage%20Type%20Object%20Reference) (InstigatedBy :type Controller%20Object%20Reference) (DamageCauser :type Actor%20Object%20Reference))
  (bind _output_get (Variables|Default|SetHealth (- (Variables|Default|GetHealth) Damage)))
  (Development|PrintString (Utilities|String|ToString(Float) _output_get))
  (if (<= _output_get 0.0)
    (Actor|DestroyActor)))

(fn ConstructionScript)