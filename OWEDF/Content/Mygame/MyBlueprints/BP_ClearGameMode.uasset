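; BP_ClearGameMode is a Blueprint, apparently the game mode for the game-clear stage, that awards a badge and shows the clear screen.
; On BeginPlay it adds the "pawre" badge uniquely to OwnedBadges on BP_MyGameInstance, stopping if that cast fails.
; It then displays WBP_CreaScreen, switches to UI-only input with a visible cursor, and prints a badge-obtained message.
; An unconnected random-chance comparison plays no part in the award.
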(event EventBeginPlay
  (bind _asbp_my_game_instance (Utilities|Casting|CastToBP_MyGameInstance (Game|GetGameInstance)))
  (Utilities|Array|AddUnique (Variables|/Game/Mygame/MyBlueprints/BP_MyGameInstance.BP_MyGameInstance_C|GetOwnedBadges _asbp_my_game_instance) "pawre")
  (bind _returnvalue (UserInterface|CreateWidget "/Game/Mygame/MyBlueprints/WBP_CreaScreen.WBP_CreaScreen_C"))
  (UserInterface|Viewport|AddtoViewport _returnvalue 0)
  (Input|SetInputModeUIOnly (Game|GetPlayerController 0) 0 "DoNotLock" (stale _output_get))
  (bind _output_get (Variables|/Script/Engine.PlayerController|SetbShowMouseCursor (Game|GetPlayerController 0) true))
  (Development|PrintString "バッジゲット"))

(fn ConstructionScript)